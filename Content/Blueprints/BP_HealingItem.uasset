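; BP_HealingItem is a reusable healing pickup that restores health to characters who touch it.
; Overlapping its sphere with an SS_BaseCharacter calls Heal on that character's HealthComponent with HealingAmount.
; It then hides its Niagara effect and disables sphere collision for CooldownTime before reactivating both.
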(event `self.ReceiveBeginPlay`)

(event `self.Sphere.OnComponentBeginOverlap`
  (params (OverlappedComponent :type "PrimitiveComponent Object Reference") (OtherActor :type "Actor Object Reference") (OtherComp :type "PrimitiveComponent Object Reference") (OtherBodyIndex :type Integer) (bFromSweep :type Boolean) (SweepResult :type "HitResult Structure (by ref)"))
  (`/Engine/EditorBlueprintResources/StandardMacros.IsValid` OtherActor
    (:`Is Valid`
      (bind _asss_base_character (cast `SS_BaseCharacter` OtherActor))
      (`self.Heal` _asss_base_character))))

(event `Heal`
  (params (CharacterToHeal :type "SS_BaseCharacter Object Reference"))
  (bind _healthcomponent (`SS_BaseCharacter.HealthComponent` CharacterToHeal)
    (:`then`
      (`SS_HealthComponent.Heal` _healthcomponent (`self.HealingAmount`))
      (set `self.bIsActive` false)
      (`SceneComponent.SetVisibility` (`self.Niagara`) false false)
      (`PrimitiveComponent.SetCollisionEnabled` (`self.Sphere`) "NoCollision")
      (`KismetSystemLibrary.Delay` (`self.CooldownTime`))
      (`self.ResetHealingArea`))
    (:`else`)))

(event `ResetHealingArea`
  (set `self.bIsActive` true)
  (`SceneComponent.SetVisibility` (`self.Niagara`) true false)
  (`PrimitiveComponent.SetCollisionEnabled` (`self.Sphere`) "QueryAndPhysics"))

(fn `UserConstructionScript`)