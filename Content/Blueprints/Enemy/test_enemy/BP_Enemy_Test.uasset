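; BP_Enemy_Test is a test enemy Blueprint that shows its AI alert state through a text indicator.
; SetEnemyStatus maps the Patrol, Investigating or Combat status to a blank, question mark or exclamation mark on StatusTextRenderer, with a matching color variable for each.
; BeginPlay, overlap, Tick and the construction script are empty, so this file holds no other behavior.
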(event `self.BP_SetEnemyStatus`
  (params (NewEnemyStatus :type "ESS_EnemyStatus Enum" :default "EnemyStatus_Patrol"))
  (`TextRenderComponent.K2_SetText` (`self.StatusTextRenderer`) (select `ESS_EnemyStatus` NewEnemyStatus :`EnemyStatus_Patrol` "" :`EnemyStatus_Investigating` "?" :`EnemyStatus_Combat` "!"))
  (`TextRenderComponent.SetTextRenderColor` (`self.StatusTextRenderer`) (select `ESS_EnemyStatus` NewEnemyStatus :`EnemyStatus_Patrol` (`self.PatrolTextColor`) :`EnemyStatus_Investigating` (`self.InvestigatingTextColor`) :`EnemyStatus_Combat` (`self.CombatTextColor`))))

(fn `UserConstructionScript`)