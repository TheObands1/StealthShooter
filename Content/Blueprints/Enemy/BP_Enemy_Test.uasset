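; BP_Enemy_Test is a test enemy that displays its AI alert state and reacts to damage and death.
; Point damage is forwarded as an AI damage-sense event, with the damage causer as instigator.
; SetEnemyStatus sets the text renderer's symbol and color for Patrol, Investigating or Combat.
; On the HealthComponent's death delegate, it removes the status text, deactivates perception, then unpossesses and destroys the AI controller.
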(event `self.ReceiveBeginPlay`
  (add `self.OnTakePointDamage` (delegate `Report Point Damage`))
  (add `SS_HealthComponent.OnDeathDelegate` (`self.HealthComponent`) (delegate `BP_OnDeath`)))

(event `Report Point Damage` :!signature `self.OnTakePointDamage`
  (params (DamagedActor :type "Actor Object Reference") (Damage :type "Float (double-precision)") (InstigatedBy :type "Controller Object Reference") (HitLocation :type "Vector Structure") (FHitComponent :type "PrimitiveComponent Object Reference") (BoneName :type Name) (ShotFromDirection :type "Vector Structure") (DamageType :type "DamageType Object Reference") (DamageCauser :type "Actor Object Reference"))
  (`AISense_Damage.ReportDamageEvent` DamagedActor DamageCauser Damage HitLocation))

(event `BP_OnDeath`
  (params (HealthComponent :type "SS_HealthComponent Object Reference") (InstigatedBy :type "Controller Object Reference") (Killer :type "Actor Object Reference"))
  (`ActorComponent.K2_DestroyComponent` (`self.StatusTextRenderer`))
  (bind _asaicontroller (cast `AIController` (`self.GetController`)))
  (`ActorComponent.Deactivate` (`AIController.GetAIPerceptionComponent` _asaicontroller))
  (`Controller.UnPossess` _asaicontroller)
  (`self.K2_DestroyActor` _asaicontroller))

(event `self.ReceiveTick`
  (params (DeltaSeconds :type "Float (single-precision)")))

(event `self.BP_SetEnemyStatus`
  (params (NewEnemyStatus :type "ESS_EnemyStatus Enum" :default "EnemyStatus_Patrol"))
  (`TextRenderComponent.K2_SetText` (`self.StatusTextRenderer`) (select `ESS_EnemyStatus` NewEnemyStatus :`EnemyStatus_Patrol` "" :`EnemyStatus_Investigating` "?" :`EnemyStatus_Combat` "!"))
  (`TextRenderComponent.SetTextRenderColor` (`self.StatusTextRenderer`) (select `ESS_EnemyStatus` NewEnemyStatus :`EnemyStatus_Patrol` (`self.PatrolTextColor`) :`EnemyStatus_Investigating` (`self.InvestigatingTextColor`) :`EnemyStatus_Combat` (`self.CombatTextColor`))))

(fn `UserConstructionScript`)