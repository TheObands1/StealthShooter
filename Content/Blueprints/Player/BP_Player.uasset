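; BP_Player is the player Blueprint that handles HUD, hurt feedback and the end-of-game screen.
; BeginPlay adds W_HUD and pre-creates W_EndGameScreen, provided the game mode is BP_GameMode.
; Any HealthComponent change plays a camera shake and adds a new W_HurtScreen.
; Death stops firing, removes the HUD, disables input, then after a short delay enables the mouse and shows the end screen.
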(event `self.ReceiveBeginPlay`
  (cast `/Game/Blueprints/Core/BP_GameMode` (`GameplayStatics.GetGameMode`))
  (bind _returnvalue (`|CreateWidget` "/Game/UI/W_HUD.W_HUD_C"))
  (bind _output_get (set `self.HUDReference` _returnvalue))
  (`UserWidget.AddToViewport` _output_get 0)
  (bind _returnvalue_2 (`|CreateWidget` "/Game/UI/W_EndGameScreen.W_EndGameScreen_C"))
  (set `self.EndGameScreenReference` _returnvalue_2))

(event `ShowEndScreen`
  (`self.StopFire`)
  (bind _hudreference (`self.HUDReference`)
    (:`then`
      (`Widget.RemoveFromParent` _hudreference)
      (bind _endgamescreenreference (`self.EndGameScreenReference`)
        (:`then`
          (`self.DisableInput` null)
          (`KismetSystemLibrary.Delay` 1.0)
          (bind _asbp_pc_gameplay (cast `/Game/Blueprints/Core/BP_PC_Gameplay` (`GameplayStatics.GetPlayerController` 0)))
          (`/Game/Blueprints/Core/BP_PC_Gameplay.EnableMouse` _asbp_pc_gameplay)
          (`UserWidget.AddToViewport` _endgamescreenreference 0))
        (:`else`)))
    (:`else`)))

(event `self.HealthComponent.OnHealthChangedDelegate`
  (params (HealthComponent :type "SS_HealthComponent Object Reference") (Health :type "Float (single-precision)") (Damage :type "Float (single-precision)") (DamageType :type "DamageType Object Reference") (InstigatedBy :type "Controller Object Reference") (DamageCauser :type "Actor Object Reference"))
  (`GameplayStatics.PlayWorldCameraShake` "/Game/Effects/BP_HurtCameraShake.BP_HurtCameraShake_C" (`self.K2_GetActorLocation` (`GameplayStatics.GetPlayerCameraManager` 0)) 10.0 100.0)
  (bind _returnvalue (`|CreateWidget` "/Game/UI/W_HurtScreen.W_HurtScreen_C"))
  (`UserWidget.AddToViewport` _returnvalue 0))

(event `self.HealthComponent.OnDeathDelegate`
  (params (HealthComponent :type "SS_HealthComponent Object Reference") (InstigatedBy :type "Controller Object Reference") (Killer :type "Actor Object Reference"))
  (`self.ShowEndScreen`))

(fn `UserConstructionScript`)