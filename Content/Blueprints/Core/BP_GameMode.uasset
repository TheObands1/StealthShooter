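; BP_GameMode is the game mode that tracks elapsed play time in minutes and seconds and handles the win state.
; Tick calls Timer until the game ends, relying on Delay to limit increments to about one per second, and broadcasts the time every frame.
; Win flags victory, broadcasts the final time, sets the ended flag and tells BP_Player to show the end screen, while GameOver is empty.
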(event `self.ReceiveTick`
  (params (DeltaSeconds :type "Float (single-precision)"))
  (if (not (`self.bHasTheGameEnded`))
    (`self.Timer`)
    (`self.BP_OnUpdateTimerDelegate` (`self.Seconds`) (`self.Minutes`))))

(event `Timer`
  (`KismetSystemLibrary.Delay` 1.0)
  (if (== (`self.Seconds`) 59)
    (set `self.Minutes` (+ (`self.Minutes`) 1))
    (set `self.Seconds` 0)
    (else
      (set `self.Seconds` (+ (`self.Seconds`) 1)))))

(event `self.BP_Win`
  (set `self.bHasPlayerWon` true)
  (`self.UpdateTimer`)
  (bind _asbp_player (cast `/Game/Blueprints/Player/BP_Player` (`GameplayStatics.GetPlayerPawn` 0)))
  (`/Game/Blueprints/Player/BP_Player.ShowEndScreen` _asbp_player))

(event `UpdateTimer`
  (`self.BP_OnUpdateTimerDelegate` (`self.Seconds`) (`self.Minutes`))
  (set `self.bHasTheGameEnded` true))

(event `self.BP_GameOver`)

(fn `UserConstructionScript`)